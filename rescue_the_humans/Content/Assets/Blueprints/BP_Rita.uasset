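; BP_Rita is a player-controlled 2D sprite pawn with four-directional idle and move flipbook animations.
; MoveUp and MoveRight axis inputs add movement along world Z and X.
; Every Tick, SetFlipbook updates the last move direction from input, with vertical taking priority over horizontal.
; It then picks the move or idle flipbook for that direction based on whether velocity is non-zero, so Rita keeps her facing when stopped.
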(event `InputAxis|MoveUp`
  (params (AxisValue :type "Float (single-precision)"))
  (`self.AddMovementInput` (0.0 0.0 1.0) AxisValue))

(event `InputAxis|MoveRight`
  (params (AxisValue :type "Float (single-precision)"))
  (`self.AddMovementInput` (1.0 0.0 0.0) AxisValue))

(event `self.ReceiveTick`
  (params (DeltaSeconds :type "Float (single-precision)"))
  (`self.SetFlipbook`))

(fn `SetFlipbook`
  (bind _lastmovedirection (`self.LastMoveDirection`))
  (if (or (!= (`self.GetInputAxisValue`) 0.0) (!= (`self.GetInputAxisValue`) 0.0))
    (set `self.LastMoveDirection` (select `bool` (> (`self.GetInputAxisValue`) 0.0) :`false` (select `bool` (< (`self.GetInputAxisValue`) 0.0) :`false` (select `bool` (> (`self.GetInputAxisValue`) 0.0) :`false` "NewEnumerator2" :`true` "NewEnumerator3" :!type "/Game/Assets/Blueprints/Move_Direction Enum") :`true` "NewEnumerator1") :`true` "NewEnumerator0")))
  (`PaperFlipbookComponent.SetFlipbook` (`self.Sprite`) (select `bool` (> (`KismetMathLibrary.VSize` (`self.GetVelocity`)) 0.0) :`false` (select `/Game/Assets/Blueprints/Move_Direction` _lastmovedirection :`NewEnumerator0` "/Game/Assets/Sprites/Rita/FB_Rita_Idle_Up.FB_Rita_Idle_Up" :`NewEnumerator1` "/Game/Assets/Sprites/Rita/FB_Rita_Idle_Down.FB_Rita_Idle_Down" :`NewEnumerator2` "/Game/Assets/Sprites/Rita/FB_Rita_Idle_Left.FB_Rita_Idle_Left" :`NewEnumerator3` "/Game/Assets/Sprites/Rita/FB_Rita_Idle_Right.FB_Rita_Idle_Right" :!type "PaperFlipbook Object Reference") :`true` (select `/Game/Assets/Blueprints/Move_Direction` _lastmovedirection :`NewEnumerator0` "/Game/Assets/Sprites/Rita/FB_Rita_Move_Up.FB_Rita_Move_Up" :`NewEnumerator1` "/Game/Assets/Sprites/Rita/FB_Rita_Move_Down.FB_Rita_Move_Down" :`NewEnumerator2` "/Game/Assets/Sprites/Rita/FB_RIta_Move_Left.FB_RIta_Move_Left" :`NewEnumerator3` "/Game/Assets/Sprites/Rita/FB_Rita_Move_Right.FB_Rita_Move_Right" :!type "PaperFlipbook Object Reference"))))

(fn `UserConstructionScript`)